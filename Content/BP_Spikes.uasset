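; BP_Spikes is a spike trap hazard that kills the player and restarts the level.
; An ActivationCollision overlap with BP_Player plays the trap's activation animation once.
; A DangerCollision overlap with BP_Player disables the player's movement, plays a death animation and game-over sound, then runs the RestartLevel console command after a short delay.
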(event `self.ActivationCollision.OnComponentBeginOverlap`
  (params (OverlappedComponent :type "PrimitiveComponent Object Reference") (OtherActor :type "Actor Object Reference") (OtherComp :type "PrimitiveComponent Object Reference") (OtherBodyIndex :type Integer) (bFromSweep :type Boolean) (SweepResult :type "HitResult Structure (by ref)"))
  (cast `/Game/BP_Player` OtherActor)
  (`SkeletalMeshComponent.PlayAnimation` (`self.Mesh`) "/Game/PlatformerAssets/Interactable/Hazard_SpikeTrap_Anim_Hazard_SpikeTrap_Armature_SpikeTrap_Activate.Hazard_SpikeTrap_Anim_Hazard_SpikeTrap_Armature_SpikeTrap_Activate" false))

(event `self.DangerCollision.OnComponentBeginOverlap`
  (params (OverlappedComponent :type "PrimitiveComponent Object Reference") (OtherActor :type "Actor Object Reference") (OtherComp :type "PrimitiveComponent Object Reference") (OtherBodyIndex :type Integer) (bFromSweep :type Boolean) (SweepResult :type "HitResult Structure (by ref)"))
  (bind _asbp_player (cast `/Game/BP_Player` OtherActor))
  (`CharacterMovementComponent.DisableMovement` (`Character.CharacterMovement` _asbp_player))
  (`SkeletalMeshComponent.PlayAnimation` (`Character.Mesh` _asbp_player) "/Game/PlatformerAssets/Player/Character_Anim_CharacterArmature_Death.Character_Anim_CharacterArmature_Death" false)
  (`GameplayStatics.PlaySound2D` "/Game/PlatformerAssets/Sounds/GameOverSound.GameOverSound" 1.0 1.0 0.0 null null)
  (`KismetSystemLibrary.Delay` 1.3)
  (`KismetSystemLibrary.ExecuteConsoleCommand` "RestartLevel" null))

(fn `UserConstructionScript`)